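; BP_CreepyFollower is an enemy pawn that chases the BP_FirstPersonCreepyFollower player and self-destructs on contact.
; Pawn sensing triggers an AI move toward that player when seen.
; Hit and overlap events both call TakeDamage on the player, then share one sequence that spawns an explosion effect and sound at the mesh and destroys the follower.
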(event `self.PawnSensing.OnSeePawn`
  (params (Pawn :type "Pawn Object Reference"))
  (bind _asbp_first_person_creepy_follower (cast `/Game/KoC/Blueprints/CreepyFollower/BP_FirstPersonCreepyFollower` Pawn))
  (`|AIMoveTo` self (0.0 0.0 0.0) _asbp_first_person_creepy_follower))

(event `self.ReceiveHit`
  (params (MyComp :type "PrimitiveComponent Object Reference") (Other :type "Actor Object Reference") (OtherComp :type "PrimitiveComponent Object Reference") (bSelfMoved :type Boolean) (HitLocation :type "Vector Structure") (HitNormal :type "Vector Structure") (NormalImpulse :type "Vector Structure") (Hit :type "HitResult Structure (by ref)"))
  (bind _returnvalue (`SceneComponent.K2_GetComponentLocation` (`self.Mesh`)))
  (bind _asbp_first_person_creepy_follower (cast `/Game/KoC/Blueprints/CreepyFollower/BP_FirstPersonCreepyFollower` Other))
  (`/Game/KoC/Blueprints/CreepyFollower/BP_FirstPersonCreepyFollower.TakeDamage` _asbp_first_person_creepy_follower)
  (`GameplayStatics.SpawnEmitterAtLocation` "/Game/StarterContent/Particles/P_Explosion.P_Explosion" _returnvalue :!label _label)
  (`GameplayStatics.PlaySoundAtLocation` "/Game/StarterContent/Audio/Explosion01.Explosion01" _returnvalue)
  (`self.K2_DestroyActor`))

(event `self.ReceiveActorBeginOverlap`
  (params (OtherActor :type "Actor Object Reference"))
  (bind _asbp_first_person_creepy_follower (cast `/Game/KoC/Blueprints/CreepyFollower/BP_FirstPersonCreepyFollower` OtherActor))
  (`/Game/KoC/Blueprints/CreepyFollower/BP_FirstPersonCreepyFollower.TakeDamage` _asbp_first_person_creepy_follower)
  (goto _label))

(fn `UserConstructionScript`)