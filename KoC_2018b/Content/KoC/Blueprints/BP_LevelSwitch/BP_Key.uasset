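; BP_Key is a key actor that opens tagged doorways when touched by an actor implementing BP_Functionality_Int.
; On overlap it plays an explosion particle effect and a collapse sound at its location.
; It then searches all BP_DoorWay actors for the ActorToAffect tag and calls OpenDoor on each match.
; The key destroys itself inside that match branch, so it remains if no doorway has the tag.
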(event `self.ReceiveActorBeginOverlap`
  (params (OtherActor :type "Actor Object Reference"))
  (bind _returnvalue (`self.K2_GetActorLocation`))
  (if (`KismetSystemLibrary.DoesImplementInterface` OtherActor "/Game/KoC/Blueprints/BP_Functionality_Int.BP_Functionality_Int_C")
    (`GameplayStatics.SpawnEmitterAtLocation` "/Game/StarterContent/Particles/P_Explosion.P_Explosion" _returnvalue)
    (`GameplayStatics.PlaySoundAtLocation` "/Game/StarterContent/Audio/Collapse01.Collapse01" _returnvalue)
    (bind _outactors (`GameplayStatics.GetAllActorsOfClass` "/Game/KoC/Blueprints/BP_LevelSwitch/BP_DoorWay.BP_DoorWay_C"))
    (for _array_element _outactors
      (if (`self.ActorHasTag` _array_element (`self.ActorToAffect`))
        (`/Game/KoC/Blueprints/BP_LevelSwitch/BP_DoorWay.OpenDoor` _array_element)
        (`self.K2_DestroyActor`)))))

(fn `UserConstructionScript`)