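; BP_DoorWay is a level-switch doorway that opens the level named by LevelToOpen when the player walks into it.
; The construction script writes that level name onto the DoorName text, so each placed door labels its destination.
; On actor overlap, only a BP_FirstPerson triggers the OpenMap function, which loads the level by name.
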(event `self.ReceiveActorBeginOverlap`
  (params (OtherActor :type "Actor Object Reference"))
  (cast `/Game/KoC/Blueprints/BP_FirstPerson/BP_FirstPerson` OtherActor)
  (`self.OpenMap` (`self.LevelToOpen`)))

(fn `OpenMap`
  (params (MapName :type Name))
  (`GameplayStatics.OpenLevel` MapName)
  (return))

(fn `UserConstructionScript`
  (`TextRenderComponent.K2_SetText` (`self.DoorName`) (`KismetTextLibrary.Conv_NameToText` (`self.LevelToOpen`))))