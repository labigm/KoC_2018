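; BP_CreepyFollower is an enemy pawn that chases the player on sight and costs them a life on contact.
; While alive, PawnSensing sends it after any seen pawn implementing BP_Functionality_Int via AIMoveTo.
; A qualifying hit calls TakeLife through a BP_ThirdPerson cast, then the follower plays a death animation, clears IsAlive and retargets AIMoveTo to itself to halt pursuit.
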(event `self.ReceiveHit`
  (params (MyComp :type "PrimitiveComponent Object Reference") (Other :type "Actor Object Reference") (OtherComp :type "PrimitiveComponent Object Reference") (bSelfMoved :type Boolean) (HitLocation :type "Vector Structure") (HitNormal :type "Vector Structure") (NormalImpulse :type "Vector Structure") (Hit :type "HitResult Structure (by ref)"))
  ;[1 1 1] If the other object is alive and implements the interface
  (if (`self.IsAlive?`)
    (if (`KismetSystemLibrary.DoesImplementInterface` Other "/Game/KoC/Blueprints/BP_Functionality_Int.BP_Functionality_Int_C")
      ;[1 1 1] I will get rid of this
      (bind _asbp_third_person (cast `/Game/KoC/Blueprints/BP_ThirdPerson/BP_ThirdPerson` Other))
      (`/Game/KoC/Blueprints/BP_ThirdPerson/BP_ThirdPerson.TakeLife` _asbp_third_person)
      ;[1 1 1] Play the dead animation mark it as dead and make sure you stop following the player
      (`SkeletalMeshComponent.PlayAnimation` (`self.Mesh`) "/Game/InfinityBladeWarriors/Character/CompleteCharacters/Animations/IB_Death_3.IB_Death_3" false)
      (set `self.IsAlive?` false)
      (`|AIMoveTo` self (0.0 0.0 0.0) self))))

(event `self.PawnSensing.OnSeePawn`
  (params (Pawn :type "Pawn Object Reference"))
  ;[1 1 1] If I see the player while being alive and it implements the interface follow it
  (if (`self.IsAlive?`)
    (if (`KismetSystemLibrary.DoesImplementInterface` Pawn "/Game/KoC/Blueprints/BP_Functionality_Int.BP_Functionality_Int_C")
      (`|AIMoveTo` self (0.0 0.0 0.0) Pawn))))

(fn `UserConstructionScript`)